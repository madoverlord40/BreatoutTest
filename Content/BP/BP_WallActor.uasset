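; Wall actor for a Breakout game that redirects the ball when it hits one of three box colliders.
; Each box's hit event casts to BreakoutBall, randomly picks one of two directions, sets a new constant X/Z velocity with randomized X speed, then plays a punch sound.
; Box and Box1 each use an opposite pair of diagonals, while Box2 always sends the ball toward negative Z.
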(event OnComponentHit(Box)
  (params (HitComponent :type Primitive%20Component%20Object%20Reference) (OtherActor :type Actor%20Object%20Reference) (OtherComp :type Primitive%20Component%20Object%20Reference) (NormalImpulse :type Vector :default "0, 0, 0") (Hit :type Hit%20Result%20Structure%20%28by%20ref%29))
  (bind _asbreakout_ball (Utilities|Casting|CastToBreakoutBall OtherActor))
  (if (Math|Random|RandomBool)
    (Class|BreakoutBall|SetNewConstVelocity _asbreakout_ball (Math|Vector|MakeVector (Math|Random|RandomFloatinRange 5e+01 1.5e+02) 0.0 1.5e+02))
    (else
      (Class|BreakoutBall|SetNewConstVelocity _asbreakout_ball (Math|Vector|MakeVector (Math|Random|RandomFloatinRange -1.5e+02 -5e+01) 0.0 -1.5e+02))))
  (Audio|PlaySound2D "/Game/Developers/james/Sound/Punch_1_2_Cue.Punch_1_2_Cue" 1.0 1.0 0.0 0 0))

(event OnComponentHit(Box1)
  (params (HitComponent :type Primitive%20Component%20Object%20Reference) (OtherActor :type Actor%20Object%20Reference) (OtherComp :type Primitive%20Component%20Object%20Reference) (NormalImpulse :type Vector :default "0, 0, 0") (Hit :type Hit%20Result%20Structure%20%28by%20ref%29))
  (bind _asbreakout_ball (Utilities|Casting|CastToBreakoutBall OtherActor))
  (if (Math|Random|RandomBool)
    (Class|BreakoutBall|SetNewConstVelocity _asbreakout_ball (Math|Vector|MakeVector (Math|Random|RandomFloatinRange 5e+01 1.5e+02) 0.0 -1.5e+02))
    (else
      (Class|BreakoutBall|SetNewConstVelocity _asbreakout_ball (Math|Vector|MakeVector (Math|Random|RandomFloatinRange -1.5e+02 -5e+01) 0.0 1.5e+02))))
  (Audio|PlaySound2D "/Game/Developers/james/Sound/Punch_1_2_Cue.Punch_1_2_Cue" 1.0 1.0 0.0 0 0))

(event OnComponentHit(Box2)
  (params (HitComponent :type Primitive%20Component%20Object%20Reference) (OtherActor :type Actor%20Object%20Reference) (OtherComp :type Primitive%20Component%20Object%20Reference) (NormalImpulse :type Vector :default "0, 0, 0") (Hit :type Hit%20Result%20Structure%20%28by%20ref%29))
  (bind _asbreakout_ball (Utilities|Casting|CastToBreakoutBall OtherActor))
  (if (Math|Random|RandomBool)
    (Class|BreakoutBall|SetNewConstVelocity _asbreakout_ball (Math|Vector|MakeVector (Math|Random|RandomFloatinRange 5e+01 1.5e+02) 0.0 -1.5e+02))
    (else
      (Class|BreakoutBall|SetNewConstVelocity _asbreakout_ball (Math|Vector|MakeVector (Math|Random|RandomFloatinRange -1.5e+02 -5e+01) 0.0 -1.5e+02))))
  (Audio|PlaySound2D "/Game/Developers/james/Sound/Punch_1_2_Cue.Punch_1_2_Cue" 1.0 1.0 0.0 0 0))

(event EventBeginPlay)

(event Collision|EventActorBeginOverlap
  (params (OtherActor :type Actor%20Object%20Reference)))

(event EventTick
  (params (DeltaSeconds :type Float%20%28single-precision%29)))

(fn ConstructionScript)