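; BP_BreakoutPC is the player controller for a Breakout game, handling paddle movement and ball launch input.
; The MoveHorizontal axis applies a Z-axis impulse, scaled by Speed, to the pawn's paddle mesh, so the paddle moves by physics.
; The handler casts the player controller itself, rather than its pawn, to BP_BreakoutPawn.
; The Launch action calls CallLaunchBall once, guarded by a BallLaunched flag.
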(event Input|ActionEvents|InputActionLaunch
  (params (Key :type Key%20Structure))
  (:Pressed
    (if (not (Variables|Default|GetBall%20Launched?))
      (Variables|Default|SetBall%20Launched? true)
      (Default|CallLaunchBall))))

(event Input|AxisEvents|InputAxisMoveHorizontal
  (params (AxisValue :type Float%20%28single-precision%29))
  (bind _asbp_breakout_pawn (Utilities|Casting|CastToBP_BreakoutPawn (Game|GetPlayerController 0)))
  (Physics|AddImpulse (Variables|/Game/BP/BP_BreakoutPawn.BP_BreakoutPawn_C|GetSM_Paddle _asbp_breakout_pawn) (Math|Vector|MakeVector 0.0 0.0 (* AxisValue (Variables|Default|GetSpeed))) "None" false))

(fn ConstructionScript)